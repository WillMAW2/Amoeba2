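; BP_ObstacleGenerator is an actor that scatters randomly shaped obstacles over a grid at BeginPlay.
; A nested loop walks scaled grid cells from the actor's location, spawning BP_Obstacle where a percentage roll against Frequency passes.
; Each spawn gets random XY deviation, slight tilt and random yaw.
; Its mesh is drawn randomly from five basic shapes, first shuffled by RandomArray through random-index insertion.
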(event `self.ReceiveBeginPlay`
  (bind _scale (`self.scale`))
  (bind _positiondeviation (`self.PositionDeviation`))
  (bind _outputarray (`self.Random Array` (`|MakeArray` "/Game/AssetPacks/StarterContent/Shapes/Shape_Cube.Shape_Cube" "/Game/AssetPacks/StarterContent/Shapes/Shape_Cone.Shape_Cone" "/Game/AssetPacks/StarterContent/Shapes/Shape_Cylinder.Shape_Cylinder" "/Game/AssetPacks/StarterContent/Shapes/Shape_NarrowCapsule.Shape_NarrowCapsule" "/Game/AssetPacks/StarterContent/Shapes/Shape_Pipe.Shape_Pipe" :!type "StaticMesh Object Reference")))
  ; Nested loop
  (for _index (range (+ (`self.GridSizeY`) 1))
    (for _index_2 (range (+ (`self.GridSizeX`) 1))
      (if (> (`self.Frequency`) (`KismetMathLibrary.RandomFloatInRange` 0.0 100.0))
        ; Add random deviation to new location
        (bind _result (`/Engine/EditorBlueprintResources/StandardMacros.NegateFloat` _positiondeviation)
          (:`  `
            ; Add new location to temp variable
            (bind _output_get (set `self.Next_Position` (+ (`KismetMathLibrary.MakeVector` (* _index_2 _scale) (* _index _scale)) (`self.K2_GetActorLocation`) (`KismetMathLibrary.MakeVector` (`KismetMathLibrary.RandomFloatInRange` _result _positiondeviation) (`KismetMathLibrary.RandomFloatInRange` _result _positiondeviation)))))
            ; Make new transform from generated location/rotation
            (bind _output_get_2 (set `self.Next_Rotation` (`KismetMathLibrary.MakeRotator` (`KismetMathLibrary.RandomFloatInRange` -10.0 10.0) (`KismetMathLibrary.RandomFloatInRange` -10.0 10.0) (`KismetMathLibrary.RandomFloatInRange` 0.0 180.0))))
            ; Make an actor with a random mesh
            (bind _returnvalue (`|SpawnActorFromClass` "/Game/Game/Obstacles/BP_Obstacle.BP_Obstacle_C" (`KismetMathLibrary.MakeTransform` _output_get _output_get_2) "Undefined" "MultiplyWithRoot" null null))
            (`StaticMeshComponent.SetStaticMesh` (`/Game/Game/Obstacles/BP_Obstacle.StaticMesh` _returnvalue) (`KismetArrayLibrary.Array_Random` _outputarray))))))))

(fn `Random Array`
  (params (InputArray :type "Array of StaticMesh Object Reference"))
  (returns (OutputArray :type "Array of StaticMesh Object Reference"))
  (bind _obstacles (`self.Obstacles`))
  (for (_array_element _array_index) InputArray
    (`KismetArrayLibrary.Array_Insert` _obstacles _array_element (`KismetMathLibrary.RandomInteger` _array_index)))
  (return _obstacles))

(fn `UserConstructionScript`)